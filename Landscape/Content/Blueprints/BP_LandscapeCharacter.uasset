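; Player character Blueprint that picks up keys and offers numpad hack shortcuts for teleporting around the level.
; The Action input calls Pick on every overlapping BP_PickableKey, passing the character's player controller.
; Numpad one to four feed NavigateToHackLocation, which builds a HackTeleportLocation tag from the index and finds matching actors.
; It teleports the character to the first match's transform and aligns control rotation with it.
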(event Input|ActionEvents|InputActionAction
  (params (Key :type Key%20Structure :default "None"))
  (:Pressed
    (for _array_element (Collision|GetOverlappingActors "/Game/Blueprints/BP_PickableKey.BP_PickableKey_C" :!class /Script/Engine.Actor)
      (bind _asbp_pickable_key (Utilities|Casting|CastToBP_PickableKey _array_element))
      (bind _asplayer_controller (Utilities|Casting|CastToPlayerController (Pawn|GetController)))
      (Default|Pick _asbp_pickable_key _asplayer_controller))))

(event Input|KeyboardEvents|NumPadOne
  (params (Key :type Key%20Structure :default "None"))
  (:Pressed
    (CallFunction|NavigatetoHackLocation 1)))

(event Input|KeyboardEvents|NumPadTwo
  (params (Key :type Key%20Structure :default "None"))
  (:Pressed
    (CallFunction|NavigatetoHackLocation 2)))

(event Input|KeyboardEvents|NumPadThree
  (params (Key :type Key%20Structure :default "None"))
  (:Pressed
    (CallFunction|NavigatetoHackLocation 3)))

(event Input|KeyboardEvents|NumPadFour
  (params (Key :type Key%20Structure :default "None"))
  (:Pressed
    (CallFunction|NavigatetoHackLocation 4)))

(fn ConstructionScript
  (|CallParentFunction))

(fn NavigatetoHackLocation
  (params (Idx :type Integer))
  (bind _outactors (Actor|GetAllActorswithTag (Utilities|String|StringToName (Utilities|String|Append "HackTeleportLocation" (Utilities|String|ToString(Integer) Idx)))))
  (if (Utilities|Array|IsNotEmpty _outactors)
    (Transformation|SetActorLocationAndRotation (Transformation|GetActorLocation (Utilities|Array|Get(acopy) _outactors)) (Transformation|GetActorRotation (Utilities|Array|Get(acopy) _outactors)) false true)
    (Pawn|SetControlRotation (Pawn|GetController) (Transformation|GetActorRotation (Utilities|Array|Get(acopy) _outactors)))))