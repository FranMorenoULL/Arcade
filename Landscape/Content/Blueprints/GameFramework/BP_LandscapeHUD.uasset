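; BP_LandscapeHUD is the HUD for the Landscape game, managing its in-game widget and end-game screen.
; On BeginPlay it creates WB_LandscapeWidget for the owning player, stores it and adds it to the viewport.
; ShowKey forwards to that widget.
; ShowEndGame shows the mouse cursor, switches input to Game and UI, and adds a new WB_LandscapeEndGame widget to the viewport.
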(event Custom|ShowKey
  (Default|ShowKey (Variables|Default|GetLandscapeWdiget)))

(event Custom|ShowEndGame
  (bind _returnvalue (Game|Player|GetOwningPlayerController))
  (Variables|/Script/Engine.PlayerController|SetbShowMouseCursor _returnvalue true)
  (Input|SetInputModeGameandUI _returnvalue 0 "DoNotLock" false)
  (bind _returnvalue_2 (UserInterface|CreateWidget "/Game/Blueprints/UI/WB_LandscapeEndGame.WB_LandscapeEndGame_C" _returnvalue))
  (UserInterface|Viewport|AddtoViewport _returnvalue_2 0))

(event EventBeginPlay
  (bind _returnvalue (UserInterface|CreateWidget "/Game/Blueprints/UI/WB_LandscapeWidget.WB_LandscapeWidget_C" (Game|Player|GetOwningPlayerController)))
  (bind _output_get (Variables|Default|SetLandscapeWdiget _returnvalue))
  (UserInterface|Viewport|AddtoViewport _output_get 0))

(fn ConstructionScript)