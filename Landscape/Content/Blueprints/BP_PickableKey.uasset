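; BP_PickableKey is a key pickup actor that reveals other actors and updates the HUD when picked.
; A sphere range, sized from PickRadius in the construction script, toggles two text hints on overlap begin and end, without filtering the overlapping actor.
; The Pick event calls ShowKey on the player's BP_LandscapeHUD, unhides each actor in ActorsToShowOnPick, then destroys the key; it stops early if the HUD cast fails.
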(event OnComponentBeginOverlap(PickRange)
  (params (OverlappedComponent :type Primitive%20Component%20Object%20Reference) (OtherActor :type Actor%20Object%20Reference) (OtherComp :type Primitive%20Component%20Object%20Reference) (OtherBodyIndex :type Integer) (bFromSweep :type Boolean) (SweepResult :type Hit%20Result%20Structure%20%28by%20ref%29))
  (CallFunction|SetTextVisibility true))

(event OnComponentEndOverlap(PickRange)
  (params (OverlappedComponent :type Primitive%20Component%20Object%20Reference) (OtherActor :type Actor%20Object%20Reference) (OtherComp :type Primitive%20Component%20Object%20Reference) (OtherBodyIndex :type Integer))
  (CallFunction|SetTextVisibility false))

(event Custom|Pick
  (params (PlayerController :type Player%20Controller%20Object%20Reference))
  (bind _asbp_landscape_hud (Utilities|Casting|CastToBP_LandscapeHUD (HUD|GetHUD PlayerController)))
  (Default|ShowKey _asbp_landscape_hud)
  (for _array_element (Variables|Default|GetActorsToShowOnPick)
    (Rendering|SetActorHiddenInGame _array_element false))
  (Actor|DestroyActor))

(fn ConstructionScript
  (Components|Sphere|SetSphereRadius (Variables|Default|GetPickRange) (Variables|Default|GetPickRadius) true))

(fn SetTextVisibility
  (params (bNewVisibility :type Boolean))
  (Rendering|SetVisibility (Variables|Default|GetTextHint) bNewVisibility false)
  (Rendering|SetVisibility (Variables|Default|GetTextHint1) bNewVisibility false))

(fn SetKeyVisibility
  (params (bNewVisibility :type Boolean))
  (Rendering|SetVisibility (Variables|Default|GetKeyMesh) bNewVisibility false))